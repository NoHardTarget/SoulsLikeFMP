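; Anim notify that plays surface-specific footstep sounds for the ranged enemy during animations.
; On notify, it traces downward from the owning actor on the Visibility channel, ignoring all base enemy actors and drawing the trace for debugging.
; A hit's physical surface type selects a grass, metal, sand, wood, rock or brick cue, played at the ranged enemy's location.
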(fn `Received_Notify`
  (params (MeshComp :type "SkeletalMeshComponent Object Reference") (Animation :type "AnimSequenceBase Object Reference") (EventReference :type "AnimNotifyEventReference Structure (by ref)"))
  (returns (ReturnValue :type Boolean))
  (bind _returnvalue (`ActorComponent.GetOwner` MeshComp))
  (bind _returnvalue_2 (`Actor.K2_GetActorLocation` _returnvalue))
  (bind _outactors (`GameplayStatics.GetAllActorsOfClass` "/Game/Blueprints/AI/BaseEnemies/BP_BaseEnemy.BP_BaseEnemy_C"))
  (bind (_outhit _returnvalue_3) (`KismetSystemLibrary.LineTraceSingle` _returnvalue_2 (+ _returnvalue_2 (* (`Actor.GetActorUpVector` _returnvalue) -200.0)) "TraceTypeQuery1" false _outactors "ForDuration"))
  (if _returnvalue_3
    (bind _asbp_ranged_enemy (cast `/Game/Blueprints/AI/RangedEnemy/BP_RangedEnemy` _returnvalue))
    (switch `EPhysicalSurface` (`GameplayStatics.GetSurfaceType` _outhit)
      (:`SurfaceType1`
        (bind _returnvalue_4 (`Actor.K2_GetActorLocation` _asbp_ranged_enemy))
        (`GameplayStatics.PlaySoundAtLocation` "/Game/Audio/SFX/Footsteps_Player/Footsteps_on_Grass_1_cue.Footsteps_on_Grass_1_cue" _returnvalue_4 (struct) 1.0 1.0 0.0 null null null null))
      (:`SurfaceType2`
        (`GameplayStatics.PlaySoundAtLocation` "/Game/Audio/SFX/Footsteps_Player/Footsteps_on_Metal_1_cue.Footsteps_on_Metal_1_cue" _returnvalue_4 (struct) 1.0 1.0 0.0 null null null null))
      (:`SurfaceType3`
        (`GameplayStatics.PlaySoundAtLocation` "/Game/Audio/SFX/Footsteps_Player/Footsteps_on_Sand_1_cue.Footsteps_on_Sand_1_cue" _returnvalue_4 (struct) 1.0 1.0 0.0 null null null null))
      (:`SurfaceType4`
        (`GameplayStatics.PlaySoundAtLocation` "/Game/Audio/SFX/Footsteps_Player/Footsteps_on_Wood_1_cue.Footsteps_on_Wood_1_cue" _returnvalue_4 (struct) 1.0 1.0 0.0 null null null null))
      (:`SurfaceType5`
        (`GameplayStatics.PlaySoundAtLocation` "/Game/Audio/SFX/Footsteps_Player/Footsteps_on_Rock_1_cue.Footsteps_on_Rock_1_cue" _returnvalue_4 (struct) 1.0 1.0 0.0 null null null null))
      (:`SurfaceType6`
        (`GameplayStatics.PlaySoundAtLocation` "/Game/Audio/SFX/Footsteps_Player/Footsteps_on_Brick_1_cue.Footsteps_on_Brick_1_cue" _returnvalue_4 (struct) 1.0 1.0 0.0 null null null null))))
  (return false))