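; Animation notify that plays surface-specific footstep sounds for enemies, named for the ranged enemy.
; On notify, it line traces downward on the Visibility channel from the owner's left foot bone, with debug drawing left on.
; If the trace hits and the owner is a BP_BaseEnemy, the hit's physical surface type selects a footstep cue, played at the enemy's actor location rather than the foot.
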(fn `Received_Notify`
  (params (MeshComp :type "SkeletalMeshComponent Object Reference") (Animation :type "AnimSequenceBase Object Reference") (EventReference :type "AnimNotifyEventReference Structure (by ref)"))
  (returns (ReturnValue :type Boolean))
  (bind _returnvalue (`ActorComponent.GetOwner` MeshComp))
  (bind _returnvalue_2 (`SceneComponent.GetSocketLocation` (`Actor.RootComponent` _returnvalue) (`SkinnedMeshComponent.GetSocketBoneName` MeshComp "foot_l")))
  (bind (_outhit _returnvalue_3) (`KismetSystemLibrary.LineTraceSingle` :`Start` _returnvalue_2 :`End` (`KismetMathLibrary.MakeVector` (.x _returnvalue_2) (.y _returnvalue_2) (- (.z _returnvalue_2) 200.0)) :`TraceChannel` "TraceTypeQuery1" :`DrawDebugType` "ForDuration"))
  (if _returnvalue_3
    (bind _asbp_base_enemy (cast `/Game/Blueprints/AI/BaseEnemies/BP_BaseEnemy` _returnvalue))
    (switch `EPhysicalSurface` (`GameplayStatics.GetSurfaceType` _outhit)
      (:`SurfaceType1`
        (bind _returnvalue_4 (`Actor.K2_GetActorLocation` _asbp_base_enemy))
        (`GameplayStatics.PlaySoundAtLocation` "/Game/Audio/SFX/Footsteps_Player/Footsteps_on_Grass_1_cue.Footsteps_on_Grass_1_cue" _returnvalue_4 (struct) 1.0 1.0 0.0 null null null null))
      (:`SurfaceType2`
        (`GameplayStatics.PlaySoundAtLocation` "/Game/Audio/SFX/Footsteps_Player/Footsteps_on_Metal_1_cue.Footsteps_on_Metal_1_cue" _returnvalue_4 (struct) 1.0 1.0 0.0 null null null null))
      (:`SurfaceType3`
        (`GameplayStatics.PlaySoundAtLocation` "/Game/Audio/SFX/Footsteps_Player/Footsteps_on_Sand_1_cue.Footsteps_on_Sand_1_cue" _returnvalue_4 (struct) 1.0 1.0 0.0 null null null null))
      (:`SurfaceType4`
        (`GameplayStatics.PlaySoundAtLocation` "/Game/Audio/SFX/Footsteps_Player/Footsteps_on_Wood_1_cue.Footsteps_on_Wood_1_cue" _returnvalue_4 (struct) 1.0 1.0 0.0 null null null null))
      (:`SurfaceType5`
        (`GameplayStatics.PlaySoundAtLocation` "/Game/Audio/SFX/Footsteps_Player/Footsteps_on_Rock_1_cue.Footsteps_on_Rock_1_cue" _returnvalue_4 (struct) 1.0 1.0 0.0 null null null null))
      (:`SurfaceType6`
        (`GameplayStatics.PlaySoundAtLocation` "/Game/Audio/SFX/Footsteps_Player/Footsteps_on_Brick_1_cue.Footsteps_on_Brick_1_cue" _returnvalue_4 (struct) 1.0 1.0 0.0 null null null null)))
    (return false)))