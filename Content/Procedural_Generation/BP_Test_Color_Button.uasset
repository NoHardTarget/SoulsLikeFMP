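; BP_Test_Color_Button is an interactable test button that sets the Red flag on a referenced Portal.
; Its AreaOfEffect overlap events track whether a BP_ThirdPersonCharacter is in range and show or hide a Widget to match.
; Tick polls the player character's Edown flag and sets Portal.Red to true while in range; nothing here resets it.
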(event `self.AreaOfEffect.OnComponentBeginOverlap`
  (params (OverlappedComponent :type "PrimitiveComponent Object Reference") (OtherActor :type "Actor Object Reference") (OtherComp :type "PrimitiveComponent Object Reference") (OtherBodyIndex :type Integer) (bFromSweep :type Boolean) (SweepResult :type "HitResult Structure (by ref)"))
  (cast `/Game/EssentialAnimation/GreatSword/Blueprint/BP_ThirdPersonCharacter` OtherActor)
  (set `self.InRange` true)
  (`SceneComponent.SetVisibility` (`self.Widget`) true false))

(event `self.AreaOfEffect.OnComponentEndOverlap`
  (params (OverlappedComponent :type "PrimitiveComponent Object Reference") (OtherActor :type "Actor Object Reference") (OtherComp :type "PrimitiveComponent Object Reference") (OtherBodyIndex :type Integer))
  (cast `/Game/EssentialAnimation/GreatSword/Blueprint/BP_ThirdPersonCharacter` OtherActor)
  (set `self.InRange` false)
  (`SceneComponent.SetVisibility` (`self.Widget`) false false))

(event `self.ReceiveTick`
  (params (DeltaSeconds :type "Float (single-precision)"))
  (bind _asbp_third_person_character (cast `/Game/EssentialAnimation/GreatSword/Blueprint/BP_ThirdPersonCharacter` (`GameplayStatics.GetPlayerCharacter` 0)))
  (if (and (`/Game/EssentialAnimation/GreatSword/Blueprint/BP_ThirdPersonCharacter.Edown` _asbp_third_person_character) (`self.InRange`))
    (set `/Game/PortalSystem/Portal_BP.Red` true (`self.Portal`))))

(fn `UserConstructionScript`)