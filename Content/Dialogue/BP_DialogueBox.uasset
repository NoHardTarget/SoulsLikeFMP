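; BP_DialogueBox is a dialogue Blueprint that shows lines of text on screen through a WB_DialogueHUD widget.
; Each Talk event advances DialogueIndex, creates the HUD if needed and displays that Dialogue entry, up to a hardcoded last index.
; Leaving the DialogueBox_Coll overlap resets the index only when it sits on that last line.
; The widget removal branch is unreachable because its index check contradicts the enclosing condition.
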(event `/Game/Dialogue/BP_DialogueInterface.Talk`
  (`/Engine/EditorBlueprintResources/StandardMacros.IncrementInt` (`self.DialogueIndex`)
    (:`  `
      (if (<= (`self.DialogueIndex`) 2)
        (`self.DialogueHUD_REF`
          (:`then`
            _)
          (:`else`
            (bind _returnvalue (`|CreateWidget` "/Game/UI/HUD/Widgets/WB_DialogueHUD.WB_DialogueHUD_C" (`GameplayStatics.GetPlayerController` 0)))
            (bind _output_get (set `self.DialogueHUD_REF` _returnvalue))
            (`UserWidget.AddToViewport` _output_get 0)))
        (`TextBlock.SetText` (`/Game/UI/HUD/Widgets/WB_DialogueHUD.Dialogue_Text` (`self.DialogueHUD_REF`)) (`KismetTextLibrary.Conv_StringToText` (`|GetArrayItem` (`self.Dialogue`) (`self.DialogueIndex`))))
        (elif (== (`self.DialogueIndex`) 2)
          (`Widget.RemoveFromParent` (`self.DialogueHUD_REF`)))))))

(event `self.DialogueBox_Coll.OnComponentEndOverlap`
  (params (OverlappedComponent :type "PrimitiveComponent Object Reference") (OtherActor :type "Actor Object Reference") (OtherComp :type "PrimitiveComponent Object Reference") (OtherBodyIndex :type Integer))
  (if (== (`self.DialogueIndex`) 2)
    (set `self.DialogueIndex` -1)))

(fn `UserConstructionScript`)