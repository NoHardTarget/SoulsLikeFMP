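; Lock-on targeting component for BP_ThirdPersonCharacter that toggles, switches left or right, and steers control rotation toward the target each tick.
; A sphere trace gathers nearby BPI_Targetting actors, then Visibility-trace hits are ranked by dot product against camera forward.
; Side switching filters by hit normal against camera right, releasing the lock when none is found.
; Locking makes the character follow controller rotation; unlocking restores orient-to-movement.
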(event `self.ReceiveBeginPlay`
  (bind _asbp_third_person_character (cast `/Game/EssentialAnimation/GreatSword/Blueprint/BP_ThirdPersonCharacter` (`self.GetOwner`)))
  (set `self.CharacterRefrence` _asbp_third_person_character)
  (set `self.CameraRefrence` (`Actor.GetComponentByClass` (`self.CharacterRefrence`) "/Script/Engine.CameraComponent")))

(event `LockOn`
  (bind _closesttarget (`self.FindClosestTarget` (`self.FindActorsToLockOnto`)))
  (`/Engine/EditorBlueprintResources/StandardMacros.IsValid` _closesttarget
    (:`Is Valid`
      (set `self.LockedOnActor` _closesttarget)
      (`self.OrientCamera`)
      (set `self.LockedOn` true))))

(event `StopLockon`
  (set `self.LockedOnActor` null)
  (set `self.LockedOn` false)
  (`self.OrientMovement`))

(event `ToggleLockon`
  (if (`self.LockedOn`)
    (`self.StopLockon`)
    (else
      (`self.LockOn`))))

(event `OrientMovement`
  (bind _charactermovement (`Character.CharacterMovement` (`self.CharacterRefrence`)))
  (set `CharacterMovementComponent.bOrientRotationToMovement` true _charactermovement)
  (set `CharacterMovementComponent.bUseControllerDesiredRotation` false _charactermovement))

(event `OrientCamera`
  (bind _charactermovement (`Character.CharacterMovement` (`self.CharacterRefrence`)))
  (set `CharacterMovementComponent.bOrientRotationToMovement` false _charactermovement)
  (set `CharacterMovementComponent.bUseControllerDesiredRotation` true _charactermovement))

(event `self.ReceiveTick`
  (params (DeltaSeconds :type "Float (single-precision)"))
  (if (`self.LockedOn`)
    (`self.FaceLockedOnActor`)))

(event `LockOntoActorLeft`
  (bind _closesttarget (`self.FindClosestTargetLeft` (`self.FindActorsToLockOnto`)))
  (`/Engine/EditorBlueprintResources/StandardMacros.IsValid` (`self.LockedOnActor`)
    (:`Is Valid`
      (`/Engine/EditorBlueprintResources/StandardMacros.IsValid` _closesttarget
        (:`Is Valid`
          (set `self.LockedOnActor` _closesttarget))
        (:`Is Not Valid`
          (`self.StopLockon`))))))

(event `LockedOntoActorRight`
  (bind _closesttarget (`self.FindClosestTargetRight` (`self.FindActorsToLockOnto`)))
  (`/Engine/EditorBlueprintResources/StandardMacros.IsValid` (`self.LockedOnActor`)
    (:`Is Valid`
      (`/Engine/EditorBlueprintResources/StandardMacros.IsValid` _closesttarget
        (:`Is Valid`
          (set `self.LockedOnActor` _closesttarget))
        (:`Is Not Valid`
          (`self.StopLockon`))))))

(fn `CheckHowCloseTargetIs`
  (params (Target :type "Actor Object Reference"))
  (returns (ReturnValue :type "Float (double-precision)"))
  (return (`KismetMathLibrary.Dot_VectorVector` (`SceneComponent.GetForwardVector` (`self.CameraRefrence`)) (`KismetMathLibrary.Conv_RotatorToVector` (`KismetMathLibrary.FindLookAtRotation` (`Actor.K2_GetActorLocation` (`self.CharacterRefrence`)) (`Actor.K2_GetActorLocation` Target))))))

(fn `FaceLockedOnActor`
  (bind _returnvalue (`Pawn.GetController` (`self.CharacterRefrence`)))
  (bind _returnvalue_2 (`Controller.GetControlRotation` _returnvalue))
  (`Controller.SetControlRotation` _returnvalue (`KismetMathLibrary.MakeRotator` (.roll _returnvalue_2) (.pitch (`KismetMathLibrary.RInterpTo_Constant` _returnvalue_2 (`KismetMathLibrary.FindLookAtRotation` (`Actor.K2_GetActorLocation` (`self.CharacterRefrence`)) (- (`Actor.K2_GetActorLocation` (`self.LockedOnActor`)) (0.0 0.0 90.0))) (`GameplayStatics.GetWorldDeltaSeconds`) (`self.Interp Speed`))) (.yaw (`KismetMathLibrary.RInterpTo_Constant` _returnvalue_2 (`KismetMathLibrary.FindLookAtRotation` (`Actor.K2_GetActorLocation` (`self.CharacterRefrence`)) (- (`Actor.K2_GetActorLocation` (`self.LockedOnActor`)) (0.0 0.0 90.0))) (`GameplayStatics.GetWorldDeltaSeconds`) (`self.Interp Speed`))))))

(fn `FindActorsToLockOnto`
  (returns (TargetingActors :type "Array of Actor Object Reference"))
  (locals (PotentialTargetingActors :type "Array of Actor Object Reference"))
  (bind _returnvalue (`Actor.K2_GetActorLocation` (`self.CharacterRefrence`)))
  (bind (_outhits _returnvalue_2) (`KismetSystemLibrary.SphereTraceMultiForObjects` _returnvalue _returnvalue 700.0 (`|MakeArray` "ObjectTypeQuery7" :!type "EObjectTypeQuery Enum") false (`|MakeArray` (`self.GetOwner`))))
  (for _array_element _outhits
    (bind (_bblockinghit _binitialoverlap _time _distance _location _impactpoint _normal _impactnormal _physmat _hitactor) (`GameplayStatics.BreakHitResult` _array_element))
    (if (and _returnvalue_2 (`KismetSystemLibrary.DoesImplementInterface` _hitactor "/Game/Blueprints/Character/BPI_Targetting.BPI_Targetting_C"))
      (`KismetArrayLibrary.Array_Add` (`local.PotentialTargetingActors`) _hitactor)))
  (return (`local.PotentialTargetingActors`)))

(fn `FindClosestTarget`
  (params (Actors :type "Array of Actor Object Reference"))
  (returns (closestTarget :type "Actor Object Reference"))
  (locals (compareTargets :type "Float (double-precision)") (closeTarget :type "Actor Object Reference"))
  (for _array_element Actors
    (bind (_outhit _returnvalue) (`KismetSystemLibrary.LineTraceSingle` :`Start` (`SceneComponent.K2_GetComponentLocation` (`self.CameraRefrence`)) :`End` (`Actor.K2_GetActorLocation` _array_element) :`TraceChannel` "TraceTypeQuery1" :`DrawDebugType` "ForDuration"))
    (if _returnvalue
      (bind _returnvalue_2 (`self.CheckHowCloseTargetIs` _array_element))
      (`/Engine/EditorBlueprintResources/StandardMacros.CompareFloat` _returnvalue_2 (`local.compareTargets`)
        (:`>`
          (set `local.compareTargets` _returnvalue_2)
          (set `local.closeTarget` _array_element)))))
  (return (`local.closeTarget`)))

(fn `FindClosestTargetLeft`
  (params (Actors :type "Array of Actor Object Reference"))
  (returns (closestTarget :type "Actor Object Reference"))
  (locals (compareTargets :type "Float (double-precision)") (closeTarget :type "Actor Object Reference"))
  (for _array_element Actors
    (bind (_outhit _returnvalue) (`KismetSystemLibrary.LineTraceSingle` :`Start` (`SceneComponent.K2_GetComponentLocation` (`self.CameraRefrence`)) :`End` (`Actor.K2_GetActorLocation` _array_element) :`TraceChannel` "TraceTypeQuery1" :`DrawDebugType` "ForDuration"))
    (if (and _returnvalue (> (`KismetMathLibrary.Dot_VectorVector` (`SceneComponent.GetRightVector` (`self.CameraRefrence`)) (`.Normal` (`GameplayStatics.BreakHitResult` _outhit))) 0.0) (!= (`self.LockedOnActor`) _array_element))
      (bind _returnvalue_2 (`self.CheckHowCloseTargetIs` _array_element))
      (`/Engine/EditorBlueprintResources/StandardMacros.CompareFloat` _returnvalue_2 (`local.compareTargets`)
        (:`>`
          (set `local.compareTargets` _returnvalue_2)
          (set `local.closeTarget` _array_element)))))
  (return (`local.closeTarget`)))

(fn `FindClosestTargetRight`
  (params (Actors :type "Array of Actor Object Reference"))
  (returns (closestTarget :type "Actor Object Reference"))
  (locals (compareTargets :type "Float (double-precision)") (closeTarget :type "Actor Object Reference"))
  (for _array_element Actors
    (bind (_outhit _returnvalue) (`KismetSystemLibrary.LineTraceSingle` :`Start` (`SceneComponent.K2_GetComponentLocation` (`self.CameraRefrence`)) :`End` (`Actor.K2_GetActorLocation` _array_element) :`TraceChannel` "TraceTypeQuery1" :`DrawDebugType` "ForDuration"))
    (if (and _returnvalue (< (`KismetMathLibrary.Dot_VectorVector` (`SceneComponent.GetRightVector` (`self.CameraRefrence`)) (`.Normal` (`GameplayStatics.BreakHitResult` _outhit))) 0.0) (!= (`self.LockedOnActor`) _array_element))
      (bind _returnvalue_2 (`self.CheckHowCloseTargetIs` _array_element))
      (`/Engine/EditorBlueprintResources/StandardMacros.CompareFloat` _returnvalue_2 (`local.compareTargets`)
        (:`>`
          (set `local.compareTargets` _returnvalue_2)
          (set `local.closeTarget` _array_element)))))
  (return (`local.closeTarget`)))