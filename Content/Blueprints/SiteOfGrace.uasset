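; Site of Grace checkpoint actor that the player discovers by interacting with it.
; A box overlap shows or hides its widget component as actors enter and leave.
; Interact stores the site as the player character's CurrentSiteofGrace, then plays the StatueFound animation on a newly created discovery widget and removes it after a short delay.
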(event `/Game/UI/Menus/Inventory/Interact.Interact`
  (bind _asbp_third_person_character (cast `/Game/EssentialAnimation/GreatSword/Blueprint/BP_ThirdPersonCharacter` (`GameplayStatics.GetPlayerCharacter` 0)))
  (set `/Game/EssentialAnimation/GreatSword/Blueprint/BP_ThirdPersonCharacter.CurrentSiteofGrace` self _asbp_third_person_character)
  (bind _returnvalue (`|CreateWidget` "/Game/UI/HUD/Widgets/WB_StatueDiscovered.WB_StatueDiscovered_C"))
  (bind _output_get (set `self.StatueDiscoveredHUD_REF` _returnvalue))
  (`UserWidget.AddToViewport` _output_get 0)
  (`UserWidget.PlayAnimationForward` _output_get (`/Game/UI/HUD/Widgets/WB_StatueDiscovered.StatueFound` _output_get) 1.0 false)
  (`KismetSystemLibrary.Delay` 4.0)
  (`Widget.RemoveFromParent` _output_get))

(event `self.Box.OnComponentBeginOverlap`
  (params (OverlappedComponent :type "PrimitiveComponent Object Reference") (OtherActor :type "Actor Object Reference") (OtherComp :type "PrimitiveComponent Object Reference") (OtherBodyIndex :type Integer) (bFromSweep :type Boolean) (SweepResult :type "HitResult Structure (by ref)"))
  (`SceneComponent.SetVisibility` (`self.Widget`) true false))

(event `self.Box.OnComponentEndOverlap`
  (params (OverlappedComponent :type "PrimitiveComponent Object Reference") (OtherActor :type "Actor Object Reference") (OtherComp :type "PrimitiveComponent Object Reference") (OtherBodyIndex :type Integer))
  (`SceneComponent.SetVisibility` (`self.Widget`) false false))

(fn `UserConstructionScript`)