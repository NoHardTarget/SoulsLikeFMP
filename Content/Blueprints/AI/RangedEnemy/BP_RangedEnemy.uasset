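; Ranged enemy character that spawns a bow on BeginPlay, attaches it to a left-hand socket and supplies movement speeds and ideal combat ranges.
; Attack plays the arrow-shot montage and signals attack end when it finishes or is interrupted.
; On a montage notify, it line-traces from the bow to the AI controller's target, but an unblocked trace only prints a debug string.
; GetPathRoute is an empty stub.
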(event `/Game/Blueprints/AI/BaseEnemies/BPI_EnemyAI.Attack`
  (bind _notifyname (`|PlayMontage` (`self.Mesh`) "/Game/Animations/RangedAni/AM_ArrowShot.AM_ArrowShot")
    (:`then`
      (`self.OnAttackEnd` :!label _label))
    (:`OnInterrupted`
      (goto _label))
    (:`OnNotifyBegin`
      (switch `name` _notifyname
        (:`Fire`
          (bind _asaic_base_enemy (cast `/Game/Blueprints/AI/BaseEnemies/AIC_BaseEnemy` (`AIBlueprintHelperLibrary.GetAIController` self)))
          (bind _attack_target (`/Game/Blueprints/AI/BaseEnemies/AIC_BaseEnemy.Attack Target` _asaic_base_enemy)
            (:`then`
              (bind (_outhit _returnvalue) (`KismetSystemLibrary.LineTraceSingle` :`Start` (`self.K2_GetActorLocation` (`self.WeaponActor`)) :`End` (`self.K2_GetActorLocation` _attack_target) :`TraceChannel` "TraceTypeQuery1" :`DrawDebugType` "ForDuration"))
              (if (not _returnvalue)
                (`KismetSystemLibrary.PrintString` "Hello")))
            (:`else`)))))))

(event `self.ReceiveBeginPlay`
  (`self.EquipWeapon`))

(event `/Game/Blueprints/AI/BaseEnemies/BPI_EnemyAI.EquipWeapon`
  (bind _returnvalue (`|SpawnActorFromClass` "/Game/Blueprints/Weapons/BP_Base_Bow.BP_Base_Bow_C" (`KismetMathLibrary.MakeTransform` (0.0 0.0 0.0)) "Undefined" "MultiplyWithRoot" null null))
  (bind _output_get (set `self.WeaponActor` _returnvalue))
  (`self.K2_AttachToComponent` _output_get (`self.Mesh`) "Hand_L_Bow_socket_Real" "KeepRelative" "KeepRelative" "KeepRelative" true)
  (set `self.IsWieldingWeapon` true)
  (`self.OnEquipWeapon`))

(fn `GetIdealRange`
  (returns (AttackRadius :type "Float (double-precision)") (DefendRadius :type "Float (double-precision)"))
  (return 1000.0 1200.0))

(fn `GetPathRoute`
  (returns (PathRoute :type "/Game/Blueprints/AI/BaseEnemies/Pathing/BP_PathingRoute Object Reference"))
  (return null))

(fn `SetMovementSpeed`
  (params (Speed :type "/Game/Blueprints/AI/BaseEnemies/Enums/E_MovementSpeed Enum" :default "NewEnumerator0"))
  (returns (SpeedValue :type "Float (double-precision)"))
  (set `CharacterMovementComponent.MaxWalkSpeed` (select `/Game/Blueprints/AI/BaseEnemies/Enums/E_MovementSpeed` Speed :`NewEnumerator1` 200.0 :`NewEnumerator2` 300.0 :`NewEnumerator3` 500.0 :!type "Float (single-precision)") (`self.CharacterMovement`))
  (return 0.0))

(fn `UserConstructionScript`
  (`parent.UserConstructionScript`))