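; Melee enemy AI character that equips a sword, unequips it and attacks through animation montages.
; Montage notifies time the weapon swap, spawning the sword onto the RightHand socket or destroying it, while a wielding flag tracks state.
; Event dispatchers signal when equip and unequip montages complete, and when the attack montage completes or is interrupted.
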(event `/Game/Blueprints/AI/BaseEnemies/BPI_EnemyAI.UnequipWeapon`
  (bind _notifyname (`|PlayMontage` (`self.Mesh`) "/Game/ARPG_Warrior/Animations/AM_UnequipSword.AM_UnequipSword")
    (:`OnCompleted`
      (`self.OnUnequipWeapon`))
    (:`OnNotifyBegin`
      (switch `name` _notifyname
        (:`ReleaseSword`
          (`self.K2_DestroyActor` (`self.WeaponActor`))
          (set `self.IsWieldingWeapon` false))))))

(event `/Game/Blueprints/AI/BaseEnemies/BPI_EnemyAI.EquipWeapon`
  (set `self.IsWieldingWeapon` true)
  (bind _notifyname (`|PlayMontage` (`self.Mesh`) "/Game/ARPG_Warrior/Animations/AM_SwordEquip.AM_SwordEquip")
    (:`OnCompleted`
      (`self.OnEquipWeapon`))
    (:`OnNotifyBegin`
      (switch `name` _notifyname
        (:`Equip Sword`
          (bind _returnvalue (`|SpawnActorFromClass` "/Game/Blueprints/Weapons/BP_Base_Sword.BP_Base_Sword_C" (`self.GetTransform`) "Undefined" "MultiplyWithRoot" null null))
          (bind _output_get (set `self.WeaponActor` _returnvalue))
          (`self.K2_AttachToComponent` _output_get (`self.Mesh`) (`self.Right Hand`) "SnapToTarget" "SnapToTarget" "SnapToTarget" true))))))

(event `/Game/Blueprints/AI/BaseEnemies/BPI_EnemyAI.Attack`
  (`|PlayMontage` (`self.Mesh`) "/Game/ARPG_Warrior/Animations/ARPG_Warrior_Anim_UE_Attack_Combo1_Montage.ARPG_Warrior_Anim_UE_Attack_Combo1_Montage"
    (:`OnCompleted`
      _)
    (:`OnInterrupted`
      _))
  (`self.OnAttackEnd`))

(fn `UserConstructionScript`
  (`parent.UserConstructionScript`))