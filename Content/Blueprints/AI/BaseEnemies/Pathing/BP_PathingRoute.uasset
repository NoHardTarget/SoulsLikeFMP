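; BP_PathingRoute is a spline-based patrol route that supplies waypoints for base enemy AI pathing.
; The PathingRoute event steps PathingIndex along the Path spline points by Direction, reversing at the first and last points for a back-and-forth route.
; GetSplineWorldPosition returns the world location of the current spline point, and the route itself moves nothing.
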(event `PathingRoute`
  (bind _output_get (set `self.PathingIndex` (+ (`self.PathingIndex`) (`self.Direction`))))
  (if (== _output_get (- (`SplineComponent.GetNumberOfSplinePoints` (`self.Path`)) 1))
    (set `self.Direction` -1)
    (elif (== (`self.PathingIndex`) 0)
      (set `self.Direction` 1))))

(fn `GetSplineWorldPosition`
  (returns (Location :type "Vector Structure"))
  (return (`SplineComponent.GetLocationAtSplinePoint` (`self.Path`) (`self.PathingIndex`) "World")))

(fn `UserConstructionScript`)