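; Base enemy character that fights the player, supplying its AI with combat ranges, a patrol route and movement speeds.
; A socket sphere trace lands debounced hits, handling player blocking and the SpikeyThorns and RingOfFire relics.
; An overlap timer counts time near the player to drive the GiveMeAHug damage buff.
; Tick watches health; death refreshes lock-on, ragdolls the mesh, stops AI logic and notifies Cave_Generation.
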(event `self.ReceiveBeginPlay`
  (bind _asaic_base_enemy (cast `/Game/Blueprints/AI/BaseEnemies/AIC_BaseEnemy` (`AIBlueprintHelperLibrary.GetAIController` self)))
  (set `self.AIC Base Enemy` _asaic_base_enemy)
  (set `self.Alive` true))

(event `self.ReceiveTick`
  (params (DeltaSeconds :type "Float (single-precision)"))
  (`self.TimeInAreaCheck`)
  (if (<= (`self.Health`) 0.0)
    (bind _asbp_third_person_character (cast `/Game/EssentialAnimation/GreatSword/Blueprint/BP_ThirdPersonCharacter` (`GameplayStatics.GetPlayerCharacter` 0)))
    (`/Engine/EditorBlueprintResources/StandardMacros.DoOnce` false
      (:`Completed`
        (bind _bpc_targetingcomponent (`/Game/EssentialAnimation/GreatSword/Blueprint/BP_ThirdPersonCharacter.BPC_TargetingComponent` _asbp_third_person_character))
        (`/Game/Blueprints/Character/BPC_TargetingComponent.StopLockon` _bpc_targetingcomponent)
        (`/Game/Blueprints/Character/BPC_TargetingComponent.LockOn` _bpc_targetingcomponent)
        (`self.Death`)))))

(event `self.RelicRange.OnComponentBeginOverlap`
  (params (OverlappedComponent :type "PrimitiveComponent Object Reference") (OtherActor :type "Actor Object Reference") (OtherComp :type "PrimitiveComponent Object Reference") (OtherBodyIndex :type Integer) (bFromSweep :type Boolean) (SweepResult :type "HitResult Structure (by ref)"))
  (cast `/Game/EssentialAnimation/GreatSword/Blueprint/BP_ThirdPersonCharacter` OtherActor)
  (`KismetSystemLibrary.K2_SetTimerDelegate` (delegate `Give Me a Hug`) 1.0 true))

(event `TimeInAreaCheck`
  (if (>= (`self.TimeInArea`) 30)
    (bind _asbp_third_person_character (cast `/Game/EssentialAnimation/GreatSword/Blueprint/BP_ThirdPersonCharacter` (`GameplayStatics.GetPlayerCharacter` 0)))
    (if (`/Game/EssentialAnimation/GreatSword/Blueprint/BP_ThirdPersonCharacter.Give Me a Hug` _asbp_third_person_character)
      (set `self.HugHappened` true)
      (set `/Game/EssentialAnimation/GreatSword/Blueprint/BP_ThirdPersonCharacter.Light Attack Damage` (* (`/Game/EssentialAnimation/GreatSword/Blueprint/BP_ThirdPersonCharacter.Light Attack Damage` _asbp_third_person_character) 1.5) _asbp_third_person_character))))

(event `Give Me a Hug`
  (set `self.TimeInArea` (+ (`self.TimeInArea`) 1)))

(event `self.RelicRange.OnComponentEndOverlap`
  (params (OverlappedComponent :type "PrimitiveComponent Object Reference") (OtherActor :type "Actor Object Reference") (OtherComp :type "PrimitiveComponent Object Reference") (OtherBodyIndex :type Integer))
  (if (`self.HugHappened`)
    (bind _asbp_third_person_character (cast `/Game/EssentialAnimation/GreatSword/Blueprint/BP_ThirdPersonCharacter` OtherActor))
    (set `self.TimeInArea` 0)
    (set `/Game/EssentialAnimation/GreatSword/Blueprint/BP_ThirdPersonCharacter.Light Attack Damage` (/ (`/Game/EssentialAnimation/GreatSword/Blueprint/BP_ThirdPersonCharacter.Light Attack Damage` _asbp_third_person_character) 1.5) _asbp_third_person_character)
    (set `self.HugHappened` false)))

(event `HitResponse`
  (if (`self.Can Be Staggered`)
    (`self.PlayAnimMontage` (`self.HitReaction`))))

(event `Death`
  (bind _mesh (`self.Mesh`))
  (set `self.Alive` false)
  (`PrimitiveComponent.SetSimulatePhysics` _mesh true)
  (`PrimitiveComponent.SetCollisionEnabled` _mesh "QueryAndPhysics")
  (`BrainComponent.StopLogic` (`AIController.BrainComponent` (`self.AIC Base Enemy`)) "")
  (bind _outactors (`GameplayStatics.GetAllActorsOfClass` "/Game/Procedural_Generation/Cave_Generation.Cave_Generation_C"))
  (`/Game/Procedural_Generation/Cave_Generation.Is Enemy Dead` _outactors self))

(fn `Enemy Take Damage`
  (params (`Damage Taken` :type "Float (double-precision)"))
  (returns (NewParam :type Boolean))
  (set `self.Health` (- (`self.Health`) `Damage Taken`))
  (return false))

(fn `GetIdealRange`
  (returns (AttackRadius :type "Float (double-precision)") (DefendRadius :type "Float (double-precision)"))
  (return 150.0 350.0))

(fn `GetPathRoute`
  (returns (PathRoute :type "/Game/Blueprints/AI/BaseEnemies/Pathing/BP_PathingRoute Object Reference"))
  (return (`self.PathingRoute`)))

(fn `HitDetection`
  (bind _returnvalue (`SceneComponent.GetSocketLocation` (`self.Mesh`) (`self.In Socket Name`)))
  (bind (_outhit _returnvalue_2) (`KismetSystemLibrary.SphereTraceSingleForObjects` :`Start` _returnvalue :`End` _returnvalue :`Radius` (`self.HitRadius`) :`ObjectTypes` (`|MakeArray` "ObjectTypeQuery3" :!type "EObjectTypeQuery Enum") :`DrawDebugType` "ForDuration"))
  (if _returnvalue_2
    (bind _asbp_third_person_character (cast `/Game/EssentialAnimation/GreatSword/Blueprint/BP_ThirdPersonCharacter` (`.HitActor` (`GameplayStatics.BreakHitResult` _outhit))))
    (if (not (`self.HasBeenHit`))
      (set `self.HasBeenHit` true)
      (if (`/Game/EssentialAnimation/GreatSword/Blueprint/BP_ThirdPersonCharacter.Ring of Fire` _asbp_third_person_character)
        (set `/Game/EssentialAnimation/GreatSword/Blueprint/BP_ThirdPersonCharacter.TimesHit` (+ (`/Game/EssentialAnimation/GreatSword/Blueprint/BP_ThirdPersonCharacter.TimesHit` _asbp_third_person_character) 1) _asbp_third_person_character))
      (if (`/Game/EssentialAnimation/GreatSword/Blueprint/BP_ThirdPersonCharacter.IsBlocking` _asbp_third_person_character)
        (set `/Game/EssentialAnimation/GreatSword/Blueprint/BP_ThirdPersonCharacter.Blocked Last Attack` true _asbp_third_person_character)
        (set `/Game/EssentialAnimation/GreatSword/Blueprint/BP_ThirdPersonCharacter.Stamina` (- (`/Game/EssentialAnimation/GreatSword/Blueprint/BP_ThirdPersonCharacter.Stamina` _asbp_third_person_character) 10.0) _asbp_third_person_character)
        (bind _spikey_thorns (`/Game/EssentialAnimation/GreatSword/Blueprint/BP_ThirdPersonCharacter.Spikey Thorns` _asbp_third_person_character))
        (if _spikey_thorns
          (set `self.Health` (- (`self.Health`) 5.0))
          (`/Game/EssentialAnimation/GreatSword/Blueprint/BP_ThirdPersonCharacter.PlayerHit` _asbp_third_person_character :!label _label)
          (`KismetSystemLibrary.K2_SetTimerDelegate` (`|CreateDelegate` :!event `IsHit`) 0.5))
        (else
          (if _spikey_thorns
            (if (== (`KismetMathLibrary.RandomInteger` 5) (`KismetMathLibrary.RandomInteger` 5))
              (set `self.Health` (- (`self.Health`) 5.0))))
          (`/Game/EssentialAnimation/GreatSword/Blueprint/BP_ThirdPersonCharacter.Hurt` _asbp_third_person_character (0.0 0.0 0.0) 0 10.0)
          (goto _label))))))

(fn `IsHit`
  (set `self.HasBeenHit` false))

(fn `SetMovementSpeed`
  (params (Speed :type "/Game/Blueprints/AI/BaseEnemies/Enums/E_MovementSpeed Enum" :default "NewEnumerator0"))
  (returns (SpeedValue :type "Float (double-precision)"))
  (bind _output_get (set `CharacterMovementComponent.MaxWalkSpeed` (select `/Game/Blueprints/AI/BaseEnemies/Enums/E_MovementSpeed` Speed :`NewEnumerator1` 100.0 :`NewEnumerator2` 300.0 :`NewEnumerator3` 500.0 :!type "Float (single-precision)") (`self.CharacterMovement`)))
  (return _output_get))

(fn `UserConstructionScript`)