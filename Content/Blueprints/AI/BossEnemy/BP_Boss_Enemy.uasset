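; Boss enemy character with montage-driven melee attacks (punch, swing, kick, uppercut, swing combo, jump attack), each signaling attack end when finished or interrupted; the generic Attack event triggers the jump attack.
; The jump attack's notify launches the boss in an arc toward the player's velocity-predicted location, stopping movement on landing.
; It also supplies movement speeds and ideal ranges, and sets hand or foot sockets for the parent's hit detection.
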(event `/Game/Blueprints/AI/BaseEnemies/BPI_EnemyAI.Attack`
  (`self.JumpAttack` null))

(event `Punch`
  (params (AttackPlayer :type "Actor Object Reference"))
  (`|PlayMontage` (`self.Mesh`) "/Game/AssetsDownloaded/Characters/Boss_PlaceHolder_/Animation/Attacks/Mutant_Punch_Montage.Mutant_Punch_Montage"
    (:`OnCompleted`
      _)
    (:`OnInterrupted`
      _))
  (`self.OnAttackEnd`))

(event `Swing`
  (params (`Attack Player` :type "Actor Object Reference"))
  (`|PlayMontage` (`self.Mesh`) "/Game/AssetsDownloaded/Characters/Boss_PlaceHolder_/Animation/Attacks/Mutant_Swiping_Montage.Mutant_Swiping_Montage"
    (:`OnCompleted`
      _)
    (:`OnInterrupted`
      _))
  (`self.OnAttackEnd`))

(event `Kick`
  (`|PlayMontage` (`self.Mesh`) "/Game/AssetsDownloaded/Characters/Boss_PlaceHolder_/Animation/Attacks/Kick.Kick"
    (:`OnCompleted`
      _)
    (:`OnInterrupted`
      _))
  (`self.OnAttackEnd`))

(event `UpperCut`
  (`|PlayMontage` (`self.Mesh`) "/Game/AssetsDownloaded/Characters/Boss_PlaceHolder_/Animation/Attacks/Mutain_Uppercut.Mutain_Uppercut"
    (:`OnCompleted`
      _)
    (:`OnInterrupted`
      _))
  (`self.OnAttackEnd`))

(event `JumpAttack`
  (params (`Attack Player` :type "Actor Object Reference"))
  (bind _notifyname (`|PlayMontage` (`self.Mesh`) "/Game/AssetsDownloaded/Characters/Boss_PlaceHolder_/Animation/Attacks/Flying_Knee_Punch_Combo_Montage.Flying_Knee_Punch_Combo_Montage")
    (:`OnCompleted`
      (`self.OnAttackEnd` :!label _label))
    (:`OnInterrupted`
      (goto _label))
    (:`OnNotifyBegin`
      (switch `name` _notifyname
        (:`Jump`
          (`self.Jump to Player`))))))

(event `SwingCombo`
  (`|PlayMontage` (`self.Mesh`) "/Game/AssetsDownloaded/Characters/Boss_PlaceHolder_/Animation/Attacks/Standing_Torch_Melee_Attack_Stab_Montage.Standing_Torch_Melee_Attack_Stab_Montage"
    (:`OnCompleted`
      _)
    (:`OnInterrupted`
      _))
  (`self.OnAttackEnd`))

(event `Jump to Player`
  (bind _location (`self.CalculateFuturePlayerLocation` (`GameplayStatics.GetPlayerCharacter` 0) 1.0))
  (bind _outlaunchvelocity (`GameplayStatics.SuggestProjectileVelocity_CustomArc` (`self.K2_GetActorLocation`) (`KismetMathLibrary.MakeVector` (.x _location) (.y _location) (+ (.z _location) 100.0))))
  (`self.LaunchCharacter` _outlaunchvelocity true true)
  (add `self.LandedDelegate` (delegate `OnLand`)))

(event `OnLand` :!signature `self.LandedDelegate`
  (params (Hit :type "HitResult Structure (by ref)"))
  (remove `self.LandedDelegate` (delegate `OnLand`))
  (`MovementComponent.StopMovementImmediately` (`self.CharacterMovement`)))

(fn `CalculateFuturePlayerLocation`
  (params (Actor :type "Actor Object Reference") (Time :type "Float (double-precision)"))
  (returns (Location :type "Vector Structure"))
  (return (+ (`self.K2_GetActorLocation` Actor) (* (* (`self.GetVelocity` Actor) (1.0 1.0 0.0)) Time))))

(fn `GetIdealRange`
  (returns (AttackRadius :type "Float (double-precision)") (DefendRadius :type "Float (double-precision)"))
  (return 275.0 800.0))

(fn `HitDetection`
  (set `self.In Socket Name` "LeftHand")
  (`parent.HitDetection`))

(fn `HitDetectionRightHand`
  (set `self.In Socket Name` "RightHand")
  (`parent.HitDetection`))

(fn `HitDetectionRightKick`
  (set `self.In Socket Name` "RightFoot")
  (set `self.HurtType` 1)
  (`parent.HitDetection`)
  (set `self.HurtType` 0))

(fn `SetMovementSpeed`
  (params (Speed :type "/Game/Blueprints/AI/BaseEnemies/Enums/E_MovementSpeed Enum" :default "NewEnumerator0"))
  (returns (SpeedValue :type "Float (double-precision)"))
  (bind _output_get (set `CharacterMovementComponent.MaxWalkSpeed` (select `/Game/Blueprints/AI/BaseEnemies/Enums/E_MovementSpeed` Speed :`NewEnumerator1` 100.0 :`NewEnumerator2` 200.0 :`NewEnumerator3` 350.0 :!type "Float (single-precision)") (`self.CharacterMovement`)))
  (return _output_get))

(fn `UserConstructionScript`
  (`parent.UserConstructionScript`))