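; BP_FogGate is a boss arena barrier that seals when its trigger box is entered and clears once the linked boss dies.
; The first box overlap shows the mesh, enables its collision and creates a boss health HUD widget bound to the Boss reference.
; Tick polls the boss's health and, once it reaches zero, hides the mesh, disables collision and removes the widget, with DoOnce guarding both transitions.
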(event `self.ReceiveTick`
  (params (DeltaSeconds :type "Float (single-precision)"))
  (bind _staticmesh (`self.StaticMesh`))
  (bind _asbp_boss_enemy (cast `/Game/Blueprints/AI/BossEnemy/BP_Boss_Enemy` (`self.Boss`)))
  (if (<= (`/Game/Blueprints/AI/BaseEnemies/BP_BaseEnemy.Health` _asbp_boss_enemy) 0.0)
    (`/Engine/EditorBlueprintResources/StandardMacros.DoOnce` false
      (:`Completed`
        (`SceneComponent.SetVisibility` _staticmesh false false)
        (`PrimitiveComponent.SetCollisionEnabled` _staticmesh "NoCollision")
        (`Widget.RemoveFromParent` (stale `self.Box.OnComponentBeginOverlap` _output_get))))))

(event `self.Box.OnComponentBeginOverlap`
  (params (OverlappedComponent :type "PrimitiveComponent Object Reference") (OtherActor :type "Actor Object Reference") (OtherComp :type "PrimitiveComponent Object Reference") (OtherBodyIndex :type Integer) (bFromSweep :type Boolean) (SweepResult :type "HitResult Structure (by ref)"))
  (bind _staticmesh (`self.StaticMesh`))
  (`/Engine/EditorBlueprintResources/StandardMacros.DoOnce` false
    (:`Completed`
      (`SceneComponent.SetVisibility` _staticmesh true false)
      (`PrimitiveComponent.SetCollisionEnabled` _staticmesh "QueryAndPhysics")
      (bind _returnvalue (`|CreateWidget` "/Game/UI/HUD/Widgets/WB_BossHealthHUD.WB_BossHealthHUD_C"))
      (bind _output_get (set `self.BossHealthBar_REF` _returnvalue))
      (`UserWidget.AddToViewport` _output_get 0)
      (set `/Game/UI/HUD/Widgets/WB_BossHealthHUD.Boss_REF` (`self.Boss`) _output_get))))

(fn `UserConstructionScript`)