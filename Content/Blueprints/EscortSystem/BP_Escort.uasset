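; Escort actor that travels along a referenced spline while the player is nearby and no enemies block it.
; The first player overlap with its sphere starts a timeline, rate-scaled by a completion time, which sets location and rotation by spline distance.
; A second sphere tracks enemies in an array.
; Tick plays or stops the timeline based on player presence and whether that array is empty.
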(event `self.ReceiveBeginPlay`)

(event `MoveEscort`
  (bind _spline (`/Game/Blueprints/EscortSystem/BP_SplinePath.Spline` (`self.SplineRef`)))
  (`TimelineComponent.SetPlayRate` (`self.Move Escort T`) (/ 1.0 (`self.TimeToComplete(S)`)))
  (bind (_direction _move) (`Timeline|Move Escort T` :!label _label)
    (:`Update`
      (bind _returnvalue (`KismetMathLibrary.Lerp` 0.0 (`SplineComponent.GetSplineLength` (`/Game/Blueprints/EscortSystem/BP_SplinePath.Spline` (`self.SplineRef`))) _move))
      (`self.K2_SetActorTransform` (`KismetMathLibrary.MakeTransform` (`SplineComponent.GetLocationAtDistanceAlongSpline` _spline _returnvalue "World") (`SplineComponent.GetRotationAtDistanceAlongSpline` _spline _returnvalue "World"))))))

(event `self.ReceiveTick`
  (params (DeltaSeconds :type "Float (single-precision)"))
  (if (> (`KismetArrayLibrary.Array_Length` (`self.EnemyArray`)) 0)
    (set `self.EnemyInRange` true)
    (else
      (set `self.EnemyInRange` false)))
  (if (`self.PlayerInRange`)
    (if (`self.EnemyInRange`)
      (goto _label :!via `Stop`)
      (else
        (goto _label)))
    (else
      (goto _label :!via `Stop`))))

(event `self.PlayerSphere.OnComponentBeginOverlap`
  (params (OverlappedComponent :type "PrimitiveComponent Object Reference") (OtherActor :type "Actor Object Reference") (OtherComp :type "PrimitiveComponent Object Reference") (OtherBodyIndex :type Integer) (bFromSweep :type Boolean) (SweepResult :type "HitResult Structure (by ref)"))
  (cast `/Game/EssentialAnimation/GreatSword/Blueprint/BP_ThirdPersonCharacter` OtherActor)
  (`|ExecutionSequence`
    (:`then_0`
      (`/Engine/EditorBlueprintResources/StandardMacros.DoOnce` false
        (:`Completed`
          (`self.MoveEscort`))))
    (:`then_1`
      (set `self.PlayerInRange` true))))

(event `self.PlayerSphere.OnComponentEndOverlap`
  (params (OverlappedComponent :type "PrimitiveComponent Object Reference") (OtherActor :type "Actor Object Reference") (OtherComp :type "PrimitiveComponent Object Reference") (OtherBodyIndex :type Integer))
  (cast `/Game/EssentialAnimation/GreatSword/Blueprint/BP_ThirdPersonCharacter` OtherActor)
  (set `self.PlayerInRange` false))

(event `self.EnemySphere.OnComponentBeginOverlap`
  (params (OverlappedComponent :type "PrimitiveComponent Object Reference") (OtherActor :type "Actor Object Reference") (OtherComp :type "PrimitiveComponent Object Reference") (OtherBodyIndex :type Integer) (bFromSweep :type Boolean) (SweepResult :type "HitResult Structure (by ref)"))
  (bind _asbp_base_enemy (cast `/Game/Blueprints/AI/BaseEnemies/BP_BaseEnemy` OtherActor))
  (`KismetArrayLibrary.Array_Add` (`self.EnemyArray`) _asbp_base_enemy))

(event `self.EnemySphere.OnComponentEndOverlap`
  (params (OverlappedComponent :type "PrimitiveComponent Object Reference") (OtherActor :type "Actor Object Reference") (OtherComp :type "PrimitiveComponent Object Reference") (OtherBodyIndex :type Integer))
  (bind _asbp_base_enemy (cast `/Game/Blueprints/AI/BaseEnemies/BP_BaseEnemy` OtherActor))
  (`KismetArrayLibrary.Array_RemoveItem` (`self.EnemyArray`) _asbp_base_enemy))

(fn `UserConstructionScript`)