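; GameArea is a trigger volume that announces a new area the first time the third-person character enters it.
; On box overlap, a DoOnce creates the WB_NewArea widget, sets the character's CurrentGameArea to this actor's GameArea value and plays the widget's NewArea animation.
; After a short fixed delay it removes the widget, and with no reset wired, later overlaps neither update the area nor show the banner.
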(event `self.Box.OnComponentBeginOverlap`
  (params (OverlappedComponent :type "PrimitiveComponent Object Reference") (OtherActor :type "Actor Object Reference") (OtherComp :type "PrimitiveComponent Object Reference") (OtherBodyIndex :type Integer) (bFromSweep :type Boolean) (SweepResult :type "HitResult Structure (by ref)"))
  (bind _asbp_third_person_character (cast `/Game/EssentialAnimation/GreatSword/Blueprint/BP_ThirdPersonCharacter` OtherActor))
  (`/Engine/EditorBlueprintResources/StandardMacros.DoOnce` false
    (:`Completed`
      (bind _returnvalue (`|CreateWidget` "/Game/UI/HUD/Widgets/WB_NewArea.WB_NewArea_C"))
      (bind _output_get (set `self.NewAreaHUD_REF` _returnvalue))
      (`UserWidget.AddToViewport` _output_get 0)
      (set `/Game/EssentialAnimation/GreatSword/Blueprint/BP_ThirdPersonCharacter.CurrentGameArea` (`self.GameArea`) _asbp_third_person_character)
      (`UserWidget.PlayAnimationForward` _output_get (`/Game/UI/HUD/Widgets/WB_NewArea.NewArea` _output_get) 1.0 false)
      (`KismetSystemLibrary.Delay` 4.0)
      (`Widget.RemoveFromParent` _output_get))))

(fn `UserConstructionScript`)