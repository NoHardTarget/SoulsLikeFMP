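; BP_Hitbox is a placeable hit volume that triggers a hurt reaction on any BP_ThirdPersonCharacter overlapping it.
; It calls Hurt with its own location and AttackType at zero damage.
; The construction script previews AttackType with a light or heavy material.
; After a hit it either destroys itself or, with IsReactivate set, disables collision and hides briefly before reactivating.
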(event `self.ReceiveActorBeginOverlap`
  (params (OtherActor :type "Actor Object Reference"))
  (bind _asbp_third_person_character (cast `/Game/EssentialAnimation/GreatSword/Blueprint/BP_ThirdPersonCharacter` OtherActor))
  (`/Game/EssentialAnimation/GreatSword/Blueprint/BP_ThirdPersonCharacter.Hurt` _asbp_third_person_character (`self.K2_GetActorLocation`) (`self.AttackType`) 0.0)
  (if (`self.isReactivate`)
    (`KismetSystemLibrary.PrintString` "Hit")
    (`self.SetActorEnableCollision` false)
    (`SceneComponent.SetVisibility` (`self.Hitbox`) false false)
    (`KismetSystemLibrary.Delay` 2.0)
    (`SceneComponent.SetVisibility` (`self.Hitbox`) true false)
    (`KismetSystemLibrary.Delay` 0.1)
    (`self.SetActorEnableCollision` true)
    (else
      (`self.K2_DestroyActor`))))

(fn `UserConstructionScript`
  (bind _hitbox (`self.Hitbox`))
  (`SceneComponent.SetVisibility` (`self.Hitbox`) true false)
  (if (== (`self.AttackType`) 0)
    (`PrimitiveComponent.SetMaterial` _hitbox 0 "/Game/EssentialAnimation/GreatSword/Demo/Material/MI_Hitbox_Light.MI_Hitbox_Light")
    (else
      (`PrimitiveComponent.SetMaterial` _hitbox 0 "/Game/EssentialAnimation/GreatSword/Demo/Material/MI_Hitbox_Heavy.MI_Hitbox_Heavy"))))