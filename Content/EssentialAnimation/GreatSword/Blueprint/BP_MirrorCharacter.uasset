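; BP_MirrorCharacter is a great-sword melee character that attaches its weapon mesh to the weapon_r socket at construction.
; HitDetect sphere-traces from the hand_r socket to the Ere component, applying light attack damage to BP_BaseEnemy hits and reporting it to AI perception.
; Helper functions toggle facing toward the targeting component's locked actor, snap yaw toward the control rotation and draw debug direction arrows.
; The event graph holds no logic.
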(fn `HitDetect`
  (bind (_outhit _returnvalue) (`KismetSystemLibrary.SphereTraceSingleForObjects` :`Start` (`SceneComponent.GetSocketLocation` (`self.Mesh`) "hand_r") :`End` (`SceneComponent.K2_GetComponentLocation` (`self.ere`)) :`Radius` 20.0 :`ObjectTypes` (`|MakeArray` "ObjectTypeQuery3" :!type "EObjectTypeQuery Enum") :`DrawDebugType` "ForDuration"))
  (if _returnvalue
    (bind _asbp_base_enemy (cast `/Game/Blueprints/AI/BaseEnemies/BP_BaseEnemy` (`.HitActor` (`GameplayStatics.BreakHitResult` _outhit)))
      (:`then`
        (`/Game/Blueprints/AI/BaseEnemies/BPI_EnemyAI.Enemy Take Damage` _asbp_base_enemy (`self.Light Attack Damage`))
        (`AISense_Damage.ReportDamageEvent` _asbp_base_enemy self 0.0 (`self.K2_GetActorLocation`)))
      (:`CastFailed`
        (`KismetSystemLibrary.PrintString` "fail")))))

(fn `UserConstructionScript`
  ;[1 1 1] Attach Weapon
  (`SceneComponent.K2_AttachToComponent` (`self.UE4_Weapon`) (`self.Mesh`) "weapon_r" "KeepRelative" "KeepRelative" "KeepRelative" true))